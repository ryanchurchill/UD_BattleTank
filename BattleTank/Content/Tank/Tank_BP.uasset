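; Tank Blueprint for a player-drivable tank with aiming, tracked movement and a health bar.
; BeginPlay initializes the aiming component with barrel and turret, the movement component with both tracks, and hands itself to the health bar widget.
; Input either sets each track's throttle directly or sends forward and turn intent to the movement component.
; Aim axes rotate the azimuth gimbal and spring arm, Fire triggers aiming, and Swap Cam toggles first- and third-person cameras.
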(event `self.ReceiveBeginPlay`
  ;[1 1 1] Initialization
  (`TankAimingComponent.Initialize` (`self.TankAiming`) (`self.Barrel`) (`self.Turret`))
  (`TankMovementComponent.Initialize` (`self.TankMovement`) (`self.Left Track`) (`self.Right Track`))
  (`self.InitializeHealthBar`))

(event `InputAxis|Left Track Throttle`
  (params (AxisValue :type "Float (single-precision)"))
  ;[1 1 1] Movement
  (`TankTrack.SetThrottle` (`self.Left Track`) AxisValue))

(event `InputAxis|AimAzimuth`
  (params (AxisValue :type "Float (single-precision)"))
  ;[1 1 1] Camera
  (`SceneComponent.K2_AddLocalRotation` (`self.Azimuth Gimbal`) (`KismetMathLibrary.MakeRotator` 0.0 0.0 AxisValue) false false))

(event `InputAction|Fire`
  (params (Key :type "Key Structure"))
  ;[1 1 1] Aim
  (:`Pressed`
    (`TankAimingComponent.Fire` (`self.TankAiming`))))

(event `InputAxis|Right Track Throttle`
  (params (AxisValue :type "Float (single-precision)"))
  ;[1 1 1] Movement
  (`TankTrack.SetThrottle` (`self.Right Track`) AxisValue))

(event `InputAxis|AimElevation`
  (params (AxisValue :type "Float (single-precision)"))
  ;[1 1 1] Camera
  (`SceneComponent.K2_AddLocalRotation` (`self.SpringArm`) (`KismetMathLibrary.MakeRotator` 0.0 AxisValue) false false))

(event `InputAxis|Move Forward`
  (params (AxisValue :type "Float (single-precision)"))
  ;[1 1 1] Movement
  (`TankMovementComponent.IntendMoveForward` (`self.TankMovement`) AxisValue))

(event `InputAxis|Turn Right`
  (params (AxisValue :type "Float (single-precision)"))
  ;[1 1 1] Movement
  (`TankMovementComponent.IntendTurnRight` (`self.TankMovement`) AxisValue))

(event `InputAction|Swap Cam`
  (params (Key :type "Key Structure"))
  ;[1 1 1] Camera Toggle
  (:`Pressed`
    (`ActorComponent.ToggleActive` (`self.3rdPersonCam`))
    (`ActorComponent.ToggleActive` (`self.1stPersonCam`))))

(fn `InitializeHealthBar`
  (bind _ashealth_bar (cast `/Game/UI/HealthBar` (`WidgetComponent.GetUserWidgetObject` (`self.Widget`))))
  (set `/Game/UI/HealthBar.MyTank` self _ashealth_bar))

(fn `UserConstructionScript`)